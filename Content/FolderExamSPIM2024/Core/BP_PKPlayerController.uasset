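; Player controller that lets the user spawn and despawn physics entities with the mouse through the PK spawning subsystem.
; On BeginPlay it enables debug and passes world bounds to the physics subsystem.
; A sphere trace under the cursor stores the hit location and flags existing entity actors.
; Left click spawns an entity there with configured transform and physics properties unless one is hit; right click despawns the hit entity.
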(event EventBeginPlay
  (bind _returnvalue (Subsystems|GetPKPhysicsSubsystem))
  (Variables|/Script/FolderExamSPIM2024.PKPhysicsSubsystem|SetbShouldDebug _returnvalue true)
  (Variables|/Script/FolderExamSPIM2024.PKPhysicsSubsystem|SetWorldBoundsMin _returnvalue (Variables|Default|GetWorld%20Bounds%20Min))
  (Variables|/Script/FolderExamSPIM2024.PKPhysicsSubsystem|SetWorldBoundsMax _returnvalue (Variables|Default|GetWorld%20Bounds%20Max)))

(event EventTick
  (params (DeltaSeconds :type Float%20%28single-precision%29)))

(event Input|MouseEvents|DebugKeyLeftMouseButton
  (params (Key :type Key%20Structure :default "None") (ActionValue :type Input%20Action%20Value%20Structure))
  (:Pressed
    (bind _shouldnotspawn (CallFunction|MouseTrace))
    (if (not _shouldnotspawn)
      (CallFunction|SpawnEntity))))

(event Input|MouseEvents|DebugKeyRightMouseButton
  (params (Key :type Key%20Structure :default "None") (ActionValue :type Input%20Action%20Value%20Structure))
  (:Pressed
    (bind (_shouldnotspawn _hitactor) (CallFunction|MouseTrace))
    (if _shouldnotspawn
      (CallFunction|DestroyEntity _hitactor))))

(fn ConstructionScript)

(fn MouseTrace
  (bind (_worldlocation _worlddirection) (Game|Player|ConvertMouseLocationToWorldSpace))
  (bind _outhit (Collision|SphereTraceByChannel _worldlocation (+ _worldlocation (* _worlddirection 1e+04)) 8e+01 "TraceTypeQuery1" false 0 "None" true "(R=1.000000,G=0.000000,B=0.000000,A=1.000000)" "(R=0.000000,G=1.000000,B=0.000000,A=1.000000)" 2.0))
  (Variables|SpawnSystem|SetEntitySpawnLocation (.Location (Collision|BreakHitResult _outhit)))
  (return (Class|GameplayStatics|ObjectIsA (.HitActor (Collision|BreakHitResult _outhit)) "/Script/FolderExamSPIM2024.PKEntityActor") (.HitActor (Collision|BreakHitResult _outhit))))

(fn SpawnEntity
  (bind _returnvalue (Subsystems|GetPKSpawningSubsystem))
  (Utilities|IsValid _returnvalue
    (:Is%20Valid
      (bind _returnvalue_2 (Class|PKSpawningSubsystem|SpawnEntityActoratLocation _returnvalue (+ (Variables|SpawnSystem|GetEntitySpawnLocation) (Math|Vector|MakeVector 0.0 0.0 -3e+01)) (Variables|SpawnSystem|GetEntitySpawnRotation) (Variables|SpawnSystem|GetEntitySpawnScale) (Variables|Default|GetEntityVelocity) (Variables|Default|GetEntityAcceleration) (Variables|Default|GetEntityMass) (Variables|Default|GetEntityCollisionRadius)))
      (Development|PrintString (Utilities|GetObjectName _returnvalue_2)))))

(fn DestroyEntity
  (params (Object :type Object%20Object%20Reference))
  (bind _returnvalue (Subsystems|GetPKSpawningSubsystem))
  (bind _aspkentity_actor (Utilities|Casting|CastToPKEntityActor Object))
  (Utilities|IsValid _returnvalue
    (:Is%20Valid
      (Class|PKSpawningSubsystem|DespawnEntityActor _returnvalue _aspkentity_actor))))